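; BP_Sphere_MovingUp is a sphere enemy variant that oscillates its mesh up and down.
; Every Tick, MovingEvent offsets the Mesh's relative Z by DirectionSpeed scaled by delta time.
; A Delay driven from Tick negates DirectionSpeed each time DirectionMoveChangeTimer elapses, reversing the movement.
; A second, parallel Delay branch multiplies the speed by one, so it has no effect.
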(event `self.ReceiveTick`
  (params (DeltaSeconds :type "Float (single-precision)"))
  (`|ExecutionSequence`
    (:`then_0`
      (`self.MovingEvent`))
    (:`then_1`
      (`KismetSystemLibrary.Delay` (`self.DirectionMoveChangeTimer`))
      (set `self.DirectionSpeed` (* (`self.DirectionSpeed`) -1.0)))
    (:`then_2`
      (`KismetSystemLibrary.Delay` (`self.DirectionMoveChangeTimer`))
      (set `self.DirectionSpeed` (* (`self.DirectionSpeed`) 1.0)))))

(event `MovingEvent`
  (`SceneComponent.K2_AddRelativeLocation` (`self.Mesh`) (`KismetMathLibrary.MakeVector` 0.0 0.0 (* (`GameplayStatics.GetWorldDeltaSeconds`) (`self.DirectionSpeed`))) false false))

(fn `UserConstructionScript`
  (`parent.UserConstructionScript`))