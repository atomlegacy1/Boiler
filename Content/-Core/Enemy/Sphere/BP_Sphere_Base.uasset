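; BP_Sphere_Base is a base sphere enemy that awards points when hit, intended as a reward for shooting it.
; Any hit on its Mesh adds SpherePoints to the FirstPersonCharacter's TotalPoints and destroys the sphere, without checking what struck it.
; A second sequence branch compares HitComponent to the player character and destroys again if they differ, which is redundant after the first destroy.
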(event `self.Mesh.OnComponentHit`
  (params (HitComponent :type "PrimitiveComponent Object Reference") (OtherActor :type "Actor Object Reference") (OtherComp :type "PrimitiveComponent Object Reference") (NormalImpulse :type "Vector Structure") (Hit :type "HitResult Structure (by ref)"))
  (bind _asfirst_person_character (cast `/Game/FirstPersonBP/Blueprints/FirstPersonCharacter` (`GameplayStatics.GetPlayerCharacter` 0) :!pure true))
  (`|ExecutionSequence`
    (:`then_0`
      ;[1 1 1] + points by shooting
      (set `/Game/FirstPersonBP/Blueprints/FirstPersonCharacter.TotalPoints` (+ (`/Game/FirstPersonBP/Blueprints/FirstPersonCharacter.TotalPoints` _asfirst_person_character) (`self.SpherePoints`)) _asfirst_person_character)
      (`self.K2_DestroyActor`))
    (:`then_1`
      (if (not (== HitComponent (`GameplayStatics.GetPlayerCharacter` 0)))
        (`self.K2_DestroyActor`)))))

(fn `UserConstructionScript`)