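; BP_RangeChecker is a component that tracks whether its owning actor is within range of player 0's character.
; Every tick it measures the distance between the two and updates the IsCatch flag.
; Separate catch and release distances allow hysteresis, so the flag sets below one threshold and clears only above the other.
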(event `self.ReceiveTick`
  (params (DeltaSeconds :type "Float (single-precision)"))
  (set `self.Distance` (`KismetMathLibrary.VSize` (- (`Actor.K2_GetActorLocation` (`self.GetOwner`)) (`Actor.K2_GetActorLocation` (`GameplayStatics.GetPlayerCharacter` 0)))))
  (if (`self.IsCatch?`)
    (if (> (`self.Distance`) (`self.ReleaseDistance`))
      (set `self.IsCatch?` false))
    (elif (< (`self.Distance`) (`self.CatchDistance`))
      (set `self.IsCatch?` true))))